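; BP_Locked is a world text indicator that shows whether its linked actor is locked.
; On Tick, after a short Delay, it casts LinkedTo to BP_Slot, falling back to BP_InteractableActor, and reads its Locked flag.
; It then sets the TextRender to a red "Locked" or a green "Unlocked" label, polling rather than reacting to lock change events.
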(event `self.ReceiveTick`
  (params (DeltaSeconds :type "Float (single-precision)"))
  ;[1 1 1] Comment
  (`KismetSystemLibrary.Delay` 0.2)
  (bind _asbp_slot (cast `/Game/Proteus_Multi/BP_Slot` (`self.LinkedTo`))
    (:`then`
      (if (`/Game/Proteus_Multi/BP_Slot.Locked` _asbp_slot)
        (`TextRenderComponent.K2_SetText` (`self.TextRender`) (`KismetTextLibrary.Conv_StringToText` "Locked") :!label _label)
        (`TextRenderComponent.SetTextRenderColor` (`self.TextRender`) (make `Color` 0 0 255 255))
        (else
          (`TextRenderComponent.K2_SetText` (`self.TextRender`) (`KismetTextLibrary.Conv_StringToText` "Unlocked") :!label _label_2)
          (`TextRenderComponent.SetTextRenderColor` (`self.TextRender`) (make `Color` 0 255 0 255)))))
    (:`CastFailed`
      (bind _asbp_interactable_actor (cast `/Game/Proteus_Multi/BP_InteractableActor` (`self.LinkedTo`)))
      (if (`/Game/Proteus_Multi/BP_InteractableActor.Locked` _asbp_interactable_actor)
        (goto _label)
        (else
          (goto _label_2))))))

(fn `UserConstructionScript`)