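; BP_Trash is a trash actor that destroys objects dropped into it.
; Its two trigger boxes, Box and Box1, each filter begin overlaps to actors implementing BI_TrashableActor, then destroy the actor after a short delay if still valid.
; Each box uses a single Delay rather than a per-actor timer, so overlaps during the wait do not get their own countdown.
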(event `self.ReceiveTick`
  (params (DeltaSeconds :type "Float (single-precision)")))

(event `self.Box.OnComponentBeginOverlap`
  (params (OverlappedComponent :type "PrimitiveComponent Object Reference") (OtherActor :type "Actor Object Reference") (OtherComp :type "PrimitiveComponent Object Reference") (OtherBodyIndex :type Integer) (bFromSweep :type Boolean) (SweepResult :type "HitResult Structure (by ref)"))
  (if (`KismetSystemLibrary.DoesImplementInterface` OtherActor "/Game/Vistom/ObjectTrash/BI_TrashableActor.BI_TrashableActor_C")
    (`KismetSystemLibrary.Delay` 3.0)
    (`/Engine/EditorBlueprintResources/StandardMacros.IsValid` OtherActor
      (:`Is Valid`
        (`self.K2_DestroyActor` OtherActor)))))

(event `self.Box1.OnComponentBeginOverlap`
  (params (OverlappedComponent :type "PrimitiveComponent Object Reference") (OtherActor :type "Actor Object Reference") (OtherComp :type "PrimitiveComponent Object Reference") (OtherBodyIndex :type Integer) (bFromSweep :type Boolean) (SweepResult :type "HitResult Structure (by ref)"))
  (if (`KismetSystemLibrary.DoesImplementInterface` OtherActor "/Game/Vistom/ObjectTrash/BI_TrashableActor.BI_TrashableActor_C")
    (`KismetSystemLibrary.Delay` 3.0)
    (`/Engine/EditorBlueprintResources/StandardMacros.IsValid` OtherActor
      (:`Is Valid`
        (`self.K2_DestroyActor` OtherActor)))))

(fn `UserConstructionScript`)