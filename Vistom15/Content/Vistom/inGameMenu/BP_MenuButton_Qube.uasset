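; BP_MenuButton_Qube is an in-game menu button labeled "Qube" that spawns an object in the world when pressed.
; It overrides the ButtonAction event from BP_ButtonParent, receiving the pressing motion controller.
; Each press spawns a BP_TrashableParent just in front of that controller, scaled down, with physics and gravity disabled.
; It then increments a counter and shows it on a text render component.
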(event `self.ButtonAction`
  (params (MotionController :type "/Game/Proteus_Multi/MotionControllerBP Object Reference"))
  (bind _motioncontoller (`self.MotionContoller`))
  ;[0 1 0.01307] Spawn Object in the world, when player pressed the button. Event Button Action comes from BP_ButtonParent
  (set `self.MotionContoller` MotionController)
  (bind _returnvalue (`|SpawnActorFromClass` "/Game/Vistom/ObjectTrash/BP_TrashableParent.BP_TrashableParent_C" (`KismetMathLibrary.Conv_VectorToTransform` (+ (`self.K2_GetActorLocation` _motioncontoller) (* (`self.GetActorForwardVector` _motioncontoller) 10.0))) "Undefined" "OverrideRootScale" null null))
  (`PrimitiveComponent.SetSimulatePhysics` (`/Game/Vistom/ObjectTrash/BP_TrashableParent.StaticMesh` _returnvalue) false)
  (`PrimitiveComponent.SetEnableGravity` (`/Game/Vistom/ObjectTrash/BP_TrashableParent.StaticMesh` _returnvalue) false)
  (`SceneComponent.SetWorldScale3D` (`Actor.RootComponent` _returnvalue) (0.25 0.25 0.25))
  (bind _output_get (set `self.Counter` (+ (`self.Counter`) 1)))
  (`TextRenderComponent.K2_SetText` (`self.TextRender1`) (`KismetTextLibrary.Conv_IntToText` _output_get)))

(fn `UserConstructionScript`
  (set `self.ButtonText` "Qube")
  (`parent.UserConstructionScript`))