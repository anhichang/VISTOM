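; BP_MenuButton is an in-game menu button that spawns a pickup object into the world when the player presses it.
; It handles the ButtonAction event from BP_ButtonParent, which supplies the pressing motion controller.
; It spawns a BP_PickupObject at the location of that controller's owner, then disables the mesh's physics simulation and gravity and shrinks its scale.
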(event `self.ButtonAction`
  (params (MotionController :type "/Game/Proteus_Multi/MotionControllerBP Object Reference"))
  ;[0 1 0.01307] Spawn Object in the world, when player pressed the button. Event Button Action comes from BP_ButtonParent
  (set `self.MotionContoller` MotionController)
  (bind _returnvalue (`|SpawnActorFromClass` "/Game/Proteus_Multi/BP_PickupObject.BP_PickupObject_C" (`KismetMathLibrary.Conv_VectorToTransform` (`self.K2_GetActorLocation` (`self.GetOwner` (`self.MotionContoller`)))) "Undefined" "OverrideRootScale" null null))
  (`PrimitiveComponent.SetSimulatePhysics` (`/Game/Proteus_Multi/BP_PickupObject.StaticMesh` _returnvalue) false)
  (`PrimitiveComponent.SetEnableGravity` (`/Game/Proteus_Multi/BP_PickupObject.StaticMesh` _returnvalue) false)
  (`SceneComponent.SetWorldScale3D` (`/Game/Proteus_Multi/BP_PickupObject.StaticMesh` _returnvalue) (0.25 0.25 0.25)))

(fn `UserConstructionScript`
  (`parent.UserConstructionScript`))