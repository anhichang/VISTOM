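; Motion-controller menu button, built on BP_ButtonParent and labelled "long profiles", that switches the in-game menu from metal to metal size.
; When pressed while the metal menu is flagged visible, it clears that flag, hides MenuMetal and shows MenuMetalSize on the left controller.
; It sets the size menu's visible flag only after a one-second delay, so that flag lags behind the visual swap.
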(event `self.ButtonAction`
  (params (MotionController :type "/Game/Proteus_Multi/MotionControllerBP Object Reference"))
  (bind _motioncontrollerleft (`/Game/Proteus_Multi/MotionControllerBP.MotionControllerLeft` (`self.MotionContoller`)))
  ;[0 1 0] Spawn Object in the world, when player pressed the button. Event Button Action comes from BP_ButtonParent
  (if (`/Game/Proteus_Multi/MotionControllerBP.IsMenu_Metal_Visible` MotionController)
    (set `self.MotionContoller` MotionController)
    (set `/Game/Proteus_Multi/MotionControllerBP.IsMenu_Metal_Visible` false (`self.MotionContoller`))
    (`SceneComponent.SetVisibility` (`/Game/Proteus_Multi/MotionControllerBP.Menu_Metal` _motioncontrollerleft) false false)
    (`SceneComponent.SetVisibility` (`/Game/Proteus_Multi/MotionControllerBP.Menu_Metal_Size` _motioncontrollerleft) true false)
    (`KismetSystemLibrary.Delay` 1.0)
    (set `/Game/Proteus_Multi/MotionControllerBP.IsMenu_Metal_Size_Visible` true (`self.MotionContoller`))))

(fn `UserConstructionScript`
  (set `self.ButtonText` "long profiles")
  (`parent.UserConstructionScript`))