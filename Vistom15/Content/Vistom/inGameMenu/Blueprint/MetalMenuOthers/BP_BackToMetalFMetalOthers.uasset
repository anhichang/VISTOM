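; A VR in-game menu button labelled "back" that returns from the Metal Others submenu to the Metal menu.
; On ButtonAction, if the submenu is flagged visible on the passed motion controller, it clears that flag and swaps the two menus' visibility on the left controller.
; The Metal menu's visible flag is set only after a short delay, separate from the immediate visual swap.
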(event `self.ButtonAction`
  (params (MotionController :type "/Game/Proteus_Multi/MotionControllerBP Object Reference"))
  (bind _motioncontrollerleft (`/Game/Proteus_Multi/MotionControllerBP.MotionControllerLeft` (`self.RightMotionContoller`)))
  (if (`/Game/Proteus_Multi/MotionControllerBP.IsMenu_Metal_Others_Visible` MotionController)
    (set `self.RightMotionContoller` MotionController)
    (set `/Game/Proteus_Multi/MotionControllerBP.IsMenu_Metal_Others_Visible` false (`self.RightMotionContoller`))
    (`SceneComponent.SetVisibility` (`/Game/Proteus_Multi/MotionControllerBP.Menu_Metal_Others` _motioncontrollerleft) false false)
    (`SceneComponent.SetVisibility` (`/Game/Proteus_Multi/MotionControllerBP.Menu_Metal` _motioncontrollerleft) true false)
    (`KismetSystemLibrary.Delay` 1.0)
    (set `/Game/Proteus_Multi/MotionControllerBP.IsMenu_Metal_Visible` true (`self.RightMotionContoller`))))

(fn `UserConstructionScript`
  (set `self.ButtonText` "back")
  (`parent.UserConstructionScript`))