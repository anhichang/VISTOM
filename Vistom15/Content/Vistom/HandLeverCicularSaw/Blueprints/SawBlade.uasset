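; VR hand-lever circular saw blade that cuts trashable metal profile actors while running.
; Tick raises the blade from lever angle, reads power from a switch or button with emergency stop, and spins it by the speed control.
; Hand contact shows a warning material and rumbles the controller.
; A cut destroys the profile and spawns two half-scaled, physics-disabled copies of three supported classes at socket actors.
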(event `self.ReceiveBeginPlay`
  (bind _returnvalue_x (`KismetMathLibrary.BreakVector` (`SceneComponent.K2_GetComponentLocation` (`/Game/Proteus_Multi/BP_InteractableActor.Mesh` (`self.RotationSpeedSlot`)))))
  ;[1 1 1] Save the initial position of the sawblade and slider
  (set `self.StartLocation` (`SceneComponent.K2_GetComponentLocation` (`self.SawBladeMesh`)))
  (set `self.StartLocationSlider` _returnvalue_x)
  ;[1 1 1] Save the initial mesh of the blade
  (set `self.InitialSawMesh` (`PrimitiveComponent.GetMaterial` (`self.SawBladeMesh`) 0)))

(event `self.ReceiveTick`
  (params (DeltaSeconds :type "Float (single-precision)"))
  (bind _motioncontroller (`self.MotionController`))
  (bind _rotationspeedslot (`self.RotationSpeedSlot`))
  (bind _returnvalue_x (`KismetMathLibrary.BreakVector` (`SceneComponent.K2_GetComponentLocation` (`/Game/Proteus_Multi/BP_InteractableActor.Mesh` (`self.RotationSpeedSlot`)))))
  (`|ExecutionSequence`
    (:`then_0`
      ;[1 1 1] Move the sawblade up and down with the lever
      (bind _asbp_interactable_actor (cast `/Game/Proteus_Multi/BP_InteractableActor` (`self.LeverSlot`)))
      (switch `/Game/Proteus_Multi/ENUM_InteractableActorType` (`/Game/Proteus_Multi/BP_InteractableActor.Type` _asbp_interactable_actor)
        (:`NewEnumerator0`
          (`SceneComponent.K2_SetWorldLocation` (`self.SawBladeMesh`) (`KismetMathLibrary.MakeVector` (.x (`self.StartLocation`)) (.y (`self.StartLocation`)) (+ (/ (`/Game/Proteus_Multi/BP_InteractableActor.CurrentAngle` _asbp_interactable_actor) 5.0) (.z (`self.StartLocation`)))) false false))))
    (:`then_1`
      ;[1 1 1] Check if Saw is ON or OFF
      (bind _asbp_interactable_actor_2 (cast `/Game/Proteus_Multi/BP_InteractableActor` (`self.ONOFFSwitchSlot`))
        (:`then`
          (switch `/Game/Proteus_Multi/ENUM_InteractableActorType` (`/Game/Proteus_Multi/BP_InteractableActor.Type` _asbp_interactable_actor_2)
            (:`NewEnumerator0`
              (set `self.ONOFF` (>= (`/Game/Proteus_Multi/BP_InteractableActor.CumulativeAngle` _asbp_interactable_actor_2) 70.0)))))
        (:`CastFailed`
          (if (`/Game/Vistom/UniversalControlls/BP_Emergency_Button.EmergencyStop` (`self.Emergency_Button`))
            (set `self.ONOFF` false)
            (set `/Game/Vistom/UniversalControlls/BP_On_Off_Button.Running` false (`self.ONOFF_Button`))
            (set `/Game/Vistom/UniversalControlls/BP_Emergency_Button.EmergencyStop` false (`self.Emergency_Button`))
            (else
              (set `self.ONOFF` (`/Game/Vistom/UniversalControlls/BP_On_Off_Button.Running` (`self.ONOFF_Button`))))))))
    (:`then_2`
      ;[1 1 1] Make rotation if machine is ON (AddRelativeRotation durch AddWroldRotation ersetzen)
      (if (`self.ONOFF`)
        (switch `/Game/Proteus_Multi/ENUM_InteractableActorType` (`/Game/Proteus_Multi/BP_InteractableActor.Type` _rotationspeedslot)
          (:`NewEnumerator0`
            (`SceneComponent.K2_AddWorldRotation` (`self.SawBladeMesh`) (`KismetMathLibrary.MakeRotator` (* (* (`/Game/Proteus_Multi/BP_InteractableActor.CumulativeAngle` _rotationspeedslot) 5.0) DeltaSeconds)) false false))
          (:`NewEnumerator1`
            (`SceneComponent.K2_AddWorldRotation` (`self.SawBladeMesh`) (`KismetMathLibrary.MakeRotator` (* (+ (* (- _returnvalue_x (`self.StartLocationSlider`)) 10.0) 20.0) DeltaSeconds)) false false)))))
    (:`then_3`
      ;[1 1 1] Play sound when machine is running
      (if (not (`self.ONOFF`))
        (`AudioComponent.Play` (`AmbientSound.AudioComponent` (`self.soundSlot`)) 0.0)))
    (:`then_4`
      (if (`KismetSystemLibrary.IsValid` _motioncontroller)
        (`/Game/Proteus_Multi/MotionControllerBP.RumbleController` _motioncontroller 0.9)))))

(event `self.Box.OnComponentEndOverlap`
  (params (OverlappedComponent :type "PrimitiveComponent Object Reference") (OtherActor :type "Actor Object Reference") (OtherComp :type "PrimitiveComponent Object Reference") (OtherBodyIndex :type Integer)))

(event `self.SawBladeMesh.OnComponentEndOverlap`
  (params (OverlappedComponent :type "PrimitiveComponent Object Reference") (OtherActor :type "Actor Object Reference") (OtherComp :type "PrimitiveComponent Object Reference") (OtherBodyIndex :type Integer))
  ;[1 1 1] Set initial mesh to sawblade when there is no more collision with hand
  (cast `/Game/Proteus_Multi/MotionControllerBP` OtherActor)
  (set `self.MotionController` null)
  (`PrimitiveComponent.SetMaterial` (`self.SawBladeMesh`) 0 (`self.InitialSawMesh`)))

(event `self.SawBladeMesh.OnComponentBeginOverlap`
  (params (OverlappedComponent :type "PrimitiveComponent Object Reference") (OtherActor :type "Actor Object Reference") (OtherComp :type "PrimitiveComponent Object Reference") (OtherBodyIndex :type Integer) (bFromSweep :type Boolean) (SweepResult :type "HitResult Structure (by ref)"))
  ;[1 1 1] Change the mesh of the saw if have collision with hand.
  (bind _asmotion_controller_bp (cast `/Game/Proteus_Multi/MotionControllerBP` OtherActor))
  (set `self.MotionController` _asmotion_controller_bp)
  (`PrimitiveComponent.SetMaterial` (`self.SawBladeMesh`) 0 "/Game/Vistom/HandLeverCicularSaw/Materials/M_Warning.M_Warning"))

(event `self.Box.OnComponentBeginOverlap`
  (params (OverlappedComponent :type "PrimitiveComponent Object Reference") (OtherActor :type "Actor Object Reference") (OtherComp :type "PrimitiveComponent Object Reference") (OtherBodyIndex :type Integer) (bFromSweep :type Boolean) (SweepResult :type "HitResult Structure (by ref)"))
  (bind _returnvalue (`GameplayStatics.GetObjectClass` (`self.OtherActor`)))
  (bind _returnvalue_2 (`GameplayStatics.GetObjectClass` (`self.OtherActor`)))
  (bind _returnvalue_3 (`KismetMathLibrary.Conv_VectorToTransform` (`self.K2_GetActorLocation` (`self.SpawnSocketSlot2`))))
  (bind _returnvalue_4 (`KismetMathLibrary.Conv_VectorToTransform` (`self.K2_GetActorLocation` (`self.SpawnSocketSlot1`))))
  (if (`KismetSystemLibrary.DoesImplementInterface` OtherActor "/Game/Vistom/ObjectTrash/BI_TrashableActor.BI_TrashableActor_C")
    (if (`self.ONOFF`)
      (set `self.OtherActor` OtherActor)
      (if (`KismetSystemLibrary.DoesImplementInterface` (`self.OtherActor`) "/Game/Vistom/ObjectTrash/BI_TrashableActor.BI_TrashableActor_C")
        (`self.K2_DestroyActor` OtherActor)
        (if (== _returnvalue_2 "/Game/Vistom/Profiles/Blueprints/BP_Profile_SQ_30_30_1_5_2.BP_Profile_SQ_30_30_1_5_2_C")
          (bind _returnvalue_5 (`|SpawnActorFromClass` "/Game/Vistom/Profiles/Blueprints/BP_Profile_SQ_30_30_1_5_2.BP_Profile_SQ_30_30_1_5_2_C" _returnvalue_4 "Undefined" "OverrideRootScale" null null))
          (bind _staticmesh (`/Game/Vistom/Profiles/Blueprints/BP_Profile_SQ_30_30_1_5_2.StaticMesh` _returnvalue_5))
          (`PrimitiveComponent.SetSimulatePhysics` _staticmesh false :!label _label)
          (`PrimitiveComponent.SetSimulatePhysics` (`/Game/Vistom/Profiles/Blueprints/BP_Profile_SQ_50_50_2_5_2.StaticMesh` (stale _returnvalue_9)) false)
          (`PrimitiveComponent.SetSimulatePhysics` (`/Game/Vistom/Profiles/Blueprints/BP_Profile_T_50_50_5_2.StaticMesh` (stale _returnvalue_10)) false)
          (`PrimitiveComponent.SetEnableGravity` _staticmesh false)
          (`PrimitiveComponent.SetEnableGravity` (`/Game/Vistom/Profiles/Blueprints/BP_Profile_SQ_50_50_2_5_2.StaticMesh` (stale _returnvalue_9)) false)
          (`PrimitiveComponent.SetEnableGravity` (`/Game/Vistom/Profiles/Blueprints/BP_Profile_T_50_50_5_2.StaticMesh` (stale _returnvalue_10)) false)
          (`self.SetActorScale3D` _returnvalue_5 (1.0 0.5 1.0))
          (`self.SetActorScale3D` (stale _returnvalue_9) (1.0 0.5 1.0))
          (`self.SetActorScale3D` (stale _returnvalue_10) (1.0 0.5 1.0))
          (`self.K2_SetActorRotation` _returnvalue_5 (struct :`Yaw` 90.0) false)
          (`self.K2_SetActorRotation` (stale _returnvalue_9) (struct :`Yaw` 90.0) false)
          (`self.K2_SetActorRotation` (stale _returnvalue_10) (struct :`Yaw` 90.0) false)
          (if (== _returnvalue "/Game/Vistom/Profiles/Blueprints/BP_Profile_SQ_30_30_1_5_2.BP_Profile_SQ_30_30_1_5_2_C")
            (bind _returnvalue_6 (`|SpawnActorFromClass` "/Game/Vistom/Profiles/Blueprints/BP_Profile_SQ_30_30_1_5_2.BP_Profile_SQ_30_30_1_5_2_C" _returnvalue_3 "Undefined" "OverrideRootScale" null null))
            (bind _staticmesh_2 (`/Game/Vistom/Profiles/Blueprints/BP_Profile_SQ_30_30_1_5_2.StaticMesh` _returnvalue_6))
            (`PrimitiveComponent.SetSimulatePhysics` _staticmesh_2 false :!label _label_2)
            (`PrimitiveComponent.SetSimulatePhysics` (`/Game/Vistom/Profiles/Blueprints/BP_Profile_SQ_50_50_2_5_2.StaticMesh` (stale _returnvalue_7)) false)
            (`PrimitiveComponent.SetSimulatePhysics` (`/Game/Vistom/Profiles/Blueprints/BP_Profile_T_50_50_5_2.StaticMesh` (stale _returnvalue_8)) false)
            (`PrimitiveComponent.SetEnableGravity` _staticmesh_2 false)
            (`PrimitiveComponent.SetEnableGravity` (`/Game/Vistom/Profiles/Blueprints/BP_Profile_SQ_50_50_2_5_2.StaticMesh` (stale _returnvalue_7)) false)
            (`PrimitiveComponent.SetEnableGravity` (`/Game/Vistom/Profiles/Blueprints/BP_Profile_T_50_50_5_2.StaticMesh` (stale _returnvalue_8)) false)
            (`self.SetActorScale3D` _returnvalue_6 (1.0 0.5 1.0))
            (`self.SetActorScale3D` (stale _returnvalue_7) (1.0 0.5 1.0))
            (`self.SetActorScale3D` (stale _returnvalue_8) (1.0 0.5 1.0))
            (`self.K2_SetActorRotation` _returnvalue_6 (struct :`Yaw` 90.0) false)
            (`self.K2_SetActorRotation` (stale _returnvalue_7) (struct :`Yaw` 90.0) false)
            (`self.K2_SetActorRotation` (stale _returnvalue_8) (struct :`Yaw` 90.0) false)
            (set `self.OtherActor` null)
            (elif (== _returnvalue "/Game/Vistom/Profiles/Blueprints/BP_Profile_SQ_50_50_2_5_2.BP_Profile_SQ_50_50_2_5_2_C")
              (bind _returnvalue_7 (`|SpawnActorFromClass` "/Game/Vistom/Profiles/Blueprints/BP_Profile_SQ_50_50_2_5_2.BP_Profile_SQ_50_50_2_5_2_C" _returnvalue_3 "Undefined" "OverrideRootScale" null null))
              (goto _label_2)
              (elif (== _returnvalue "/Game/Vistom/Profiles/Blueprints/BP_Profile_T_50_50_5_2.BP_Profile_T_50_50_5_2_C")
                (bind _returnvalue_8 (`|SpawnActorFromClass` "/Game/Vistom/Profiles/Blueprints/BP_Profile_T_50_50_5_2.BP_Profile_T_50_50_5_2_C" _returnvalue_3 "Undefined" "OverrideRootScale" null null))
                (goto _label_2)
                (else
                  (set `self.OtherActor` null)))))
          (elif (== _returnvalue_2 "/Game/Vistom/Profiles/Blueprints/BP_Profile_SQ_50_50_2_5_2.BP_Profile_SQ_50_50_2_5_2_C")
            (bind _returnvalue_9 (`|SpawnActorFromClass` "/Game/Vistom/Profiles/Blueprints/BP_Profile_SQ_50_50_2_5_2.BP_Profile_SQ_50_50_2_5_2_C" _returnvalue_4 "Undefined" "OverrideRootScale" null null))
            (goto _label)
            (elif (== _returnvalue_2 "/Game/Vistom/Profiles/Blueprints/BP_Profile_T_50_50_5_2.BP_Profile_T_50_50_5_2_C")
              (bind _returnvalue_10 (`|SpawnActorFromClass` "/Game/Vistom/Profiles/Blueprints/BP_Profile_T_50_50_5_2.BP_Profile_T_50_50_5_2_C" _returnvalue_4 "Undefined" "OverrideRootScale" null null))
              (goto _label)
              (else
                (set `self.OtherActor` null)))))
        (else
          (set `self.OtherActor` null))))))

(fn `UserConstructionScript`)