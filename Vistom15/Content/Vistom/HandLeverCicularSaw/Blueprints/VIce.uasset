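; Blueprint for a vice on the hand lever circular saw that tightens as its wheel is turned.
; BeginPlay stores the vice mesh's world position.
; Every Tick it offsets the mesh along world Y from that start by the wheel slot's cumulative angle, scaled down by a fixed divisor, turning circular motion into linear travel.
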(event `self.ReceiveBeginPlay`
  ;[0 1 0.1783] Save the startposition of the vice
  (set `self.Startposition` (`SceneComponent.K2_GetComponentLocation` (`self.ViceStaticMesh`))))

(event `self.ReceiveTick`
  (params (DeltaSeconds :type "Float (single-precision)"))
  (`|ExecutionSequence`
    (:`then_0`
      ;[0 1 0] Tighten the vice according to the angle of the wheel (circular motion)
      (`SceneComponent.K2_SetWorldLocation` (`self.ViceStaticMesh`) (`KismetMathLibrary.MakeVector` (.x (`self.Startposition`)) (- (.y (`self.Startposition`)) (/ (`/Game/Proteus_Multi/BP_InteractableActor.CumulativeAngle` (`self.WheelSlot`)) 95.0)) (.z (`self.Startposition`))) false false))))

(fn `UserConstructionScript`)