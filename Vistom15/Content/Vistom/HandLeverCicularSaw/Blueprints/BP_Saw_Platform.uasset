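; BP_Saw_Platform is the platform of a hand-lever circular saw that holds a profile actor in place.
; Each SnapProfile call alternates between grab and release through a FlipFlop.
; Grab takes the first actor overlapping Box, attaches it to Platform's Snap socket keeping its world transform, and disables its collision.
; Release detaches that stored actor in place and restores its collision.
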(event `SnapProfile`
  (`/Engine/EditorBlueprintResources/StandardMacros.FlipFlop`
    (:`A`
      (set `self.Profile_Actor` (`|GetArrayItem` (`PrimitiveComponent.GetOverlappingActors` (`self.Box`) null)))
      (`self.K2_AttachToComponent` (`self.Profile_Actor`) (`self.Platform`) "Snap" "KeepWorld" "KeepWorld" "KeepWorld" true)
      (`self.SetActorEnableCollision` (`self.Profile_Actor`) false))
    (:`B`
      (`SceneComponent.K2_DetachFromComponent` (`Actor.RootComponent` (`self.Profile_Actor`)) "KeepWorld" "KeepWorld" "KeepWorld" true)
      (`self.SetActorEnableCollision` (`self.Profile_Actor`) true))))

(fn `UserConstructionScript`)