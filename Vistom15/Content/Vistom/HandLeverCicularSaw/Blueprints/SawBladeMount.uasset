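; SawBladeMount is the blade mount of a hand-lever circular saw, moving up and down as the lever rotates.
; It stores the MountMesh world location on BeginPlay as a baseline.
; Each Tick it casts LeverSlot to BP_InteractableActor and, for the Rotation type, sets the mesh height to that baseline plus the lever's scaled CurrentAngle, without sweeping.
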(event `self.ReceiveBeginPlay`
  ;[0 1 0] Save the initial position of the sawblade mount
  (set `self.StartLocation` (`SceneComponent.K2_GetComponentLocation` (`self.MountMesh`))))

(event `self.ReceiveTick`
  (params (DeltaSeconds :type "Float (single-precision)"))
  ;[0 1 0] Move the sawblade mount up and down with the lever
  (bind _asbp_interactable_actor (cast `/Game/Proteus_Multi/BP_InteractableActor` (`self.LeverSlot`)))
  (switch `/Game/Proteus_Multi/ENUM_InteractableActorType` (`/Game/Proteus_Multi/BP_InteractableActor.Type` _asbp_interactable_actor)
    (:`NewEnumerator0`
      (`SceneComponent.K2_SetWorldLocation` (`self.MountMesh`) (`KismetMathLibrary.MakeVector` (.x (`self.StartLocation`)) (.y (`self.StartLocation`)) (+ (/ (`/Game/Proteus_Multi/BP_InteractableActor.CurrentAngle` _asbp_interactable_actor) 5.0) (.z (`self.StartLocation`)))) false false))))

(fn `UserConstructionScript`)