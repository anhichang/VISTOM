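; BP_Stopper is a movable stopper for the hand lever circular saw that slides its static mesh along world X.
; It caches the mesh's world position on BeginPlay.
; MoveStopper, triggered from BP_Input_Panel, takes an absolute distance and uses a timeline to lerp X by the difference from the previous distance.
; When the timeline finishes, it stores the new position and distance as the base for the next move.
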(event `self.ReceiveBeginPlay`
  ;[0 1 0] Set the origin location of the stopper
  (set `self.StopperPosition` (`SceneComponent.K2_GetComponentLocation` (`self.StaticMesh`))))

(event `MoveStopper`
  (params (MovingDistance :type "Float (double-precision)"))
  (bind _x (.x (`self.StopperPosition`)))
  ;[0 1 0] Set the world location of the stopper. MoveStopper function will be triggered in BP_Input_Panel. The stoppers will move
  (bind (_direction _newtrack_2) (`Timeline|Timeline_0` :!via `PlayFromStart`)
    (:`Update`
      (bind _returnvalue (`KismetMathLibrary.MakeVector` (`KismetMathLibrary.Lerp` _x (+ (- MovingDistance (`self.OldDistance`)) _x) _newtrack_2) (.y (`self.StopperPosition`)) (.z (`self.StopperPosition`))))
      (`SceneComponent.K2_SetWorldLocation` (`self.StaticMesh`) _returnvalue false false))
    (:`Finished`
      (set `self.StopperPosition` _returnvalue)
      (set `self.OldDistance` MovingDistance))))

(fn `UserConstructionScript`)