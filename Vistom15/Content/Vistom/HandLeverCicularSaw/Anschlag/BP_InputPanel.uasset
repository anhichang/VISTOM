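; BP_InputPanel is a numeric keypad for the hand lever circular saw's stop (Anschlag), used to enter the position the stopper moves to.
; Digit events append to TextToShow only while the value stays within MaxLength, which caps the numeric value rather than the character count.
; Dot allows a single decimal point, clear events erase all or the last character, and each edit refreshes ConcadinatedText.
; OK passes the parsed float to StopperSlot.MoveStopper.
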(event `SetNum1`
  (bind _returnvalue (`KismetStringLibrary.Concat_StrStr` (`self.TextToShow`) "1"))
  ;[0 1 0] Mapping for input numbers
  (if (<= (`KismetStringLibrary.Conv_StringToDouble` _returnvalue) (`self.MaxLength`))
    (set `self.TextToShow` _returnvalue)
    (`TextRenderComponent.K2_SetText` (`self.ConcadinatedText`) (`KismetTextLibrary.Conv_StringToText` (`self.TextToShow`)) :!label _label)))

(event `SetOk`
  ;[0 1 0] Comment
  (`/Game/Vistom/HandLeverCicularSaw/Anschlag/BP_Stopper.MoveStopper` (`self.StopperSlot`) (`KismetStringLibrary.Conv_StringToDouble` (`self.TextToShow`))))

(event `SetNum2`
  (bind _returnvalue (`KismetStringLibrary.Concat_StrStr` (`self.TextToShow`) "2"))
  ;[0 1 0] Mapping for input numbers
  (if (<= (`KismetStringLibrary.Conv_StringToDouble` _returnvalue) (`self.MaxLength`))
    (set `self.TextToShow` _returnvalue)
    (goto _label)))

(event `SetNum6`
  (bind _returnvalue (`KismetStringLibrary.Concat_StrStr` (`self.TextToShow`) "6"))
  ;[0 1 0] Mapping for input numbers
  (if (<= (`KismetStringLibrary.Conv_StringToDouble` _returnvalue) (`self.MaxLength`))
    (set `self.TextToShow` _returnvalue)
    (goto _label)))

(event `SetNum3`
  (bind _returnvalue (`KismetStringLibrary.Concat_StrStr` (`self.TextToShow`) "3"))
  ;[0 1 0] Mapping for input numbers
  (if (<= (`KismetStringLibrary.Conv_StringToDouble` _returnvalue) (`self.MaxLength`))
    (set `self.TextToShow` _returnvalue)
    (goto _label)))

(event `SetNum7`
  (bind _returnvalue (`KismetStringLibrary.Concat_StrStr` (`self.TextToShow`) "7"))
  ;[0 1 0] Mapping for input numbers
  (if (<= (`KismetStringLibrary.Conv_StringToDouble` _returnvalue) (`self.MaxLength`))
    (set `self.TextToShow` _returnvalue)
    (goto _label)))

(event `SetNum4`
  (bind _returnvalue (`KismetStringLibrary.Concat_StrStr` (`self.TextToShow`) "4"))
  ;[0 1 0] Mapping for input numbers
  (if (<= (`KismetStringLibrary.Conv_StringToDouble` _returnvalue) (`self.MaxLength`))
    (set `self.TextToShow` _returnvalue)
    (goto _label)))

(event `SetNum8`
  (bind _returnvalue (`KismetStringLibrary.Concat_StrStr` (`self.TextToShow`) "8"))
  ;[0 1 0] Mapping for input numbers
  (if (<= (`KismetStringLibrary.Conv_StringToDouble` _returnvalue) (`self.MaxLength`))
    (set `self.TextToShow` _returnvalue)
    (goto _label)))

(event `ClearNum`
  ;[0 1 0] Mapping for other buttons
  (set `self.TextToShow` "")
  (goto _label))

(event `SetNum5`
  (bind _returnvalue (`KismetStringLibrary.Concat_StrStr` (`self.TextToShow`) "5"))
  ;[0 1 0] Mapping for input numbers
  (if (<= (`KismetStringLibrary.Conv_StringToDouble` _returnvalue) (`self.MaxLength`))
    (set `self.TextToShow` _returnvalue)
    (goto _label)))

(event `ClearLast`
  (bind _texttoshow (`self.TextToShow`))
  ;[0 1 0] Mapping for other buttons
  (set `self.TextToShow` (`KismetStringLibrary.GetSubstring` _texttoshow 0 (- (`KismetStringLibrary.Len` _texttoshow) 1)))
  (goto _label))

(event `SetNum9`
  (bind _returnvalue (`KismetStringLibrary.Concat_StrStr` (`self.TextToShow`) "9"))
  ;[0 1 0] Mapping for input numbers
  (if (<= (`KismetStringLibrary.Conv_StringToDouble` _returnvalue) (`self.MaxLength`))
    (set `self.TextToShow` _returnvalue)
    (goto _label)))

(event `SetDot`
  (bind _texttoshow (`self.TextToShow`))
  ;[0 1 0] Mapping for other buttons
  (if (not (`KismetStringLibrary.Contains` _texttoshow "."))
    (set `self.TextToShow` (`KismetStringLibrary.Concat_StrStr` _texttoshow "."))
    (goto _label)))

(event `SetNum0`
  (bind _returnvalue (`KismetStringLibrary.Concat_StrStr` (`self.TextToShow`) "0"))
  ;[0 1 0] Mapping for input numbers
  (if (<= (`KismetStringLibrary.Conv_StringToDouble` _returnvalue) (`self.MaxLength`))
    (set `self.TextToShow` _returnvalue)
    (goto _label)))

(fn `UserConstructionScript`
  (`TextRenderComponent.K2_SetText` (`self.ConcadinatedText`) (`KismetTextLibrary.Conv_StringToText` (`self.TextToShow`))))