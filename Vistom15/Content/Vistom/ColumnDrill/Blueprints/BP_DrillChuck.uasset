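; Drill chuck of a VR column drill, driven each Tick by slotted interactable controls.
; A lever's angle sets chuck height, while a rotary switch, or a run button with emergency stop, sets the on/off state.
; When on, it spins at a speed taken from a dial or slider.
; Motion controllers entering its box swap in a warning material; the sound's Play call fires while off, despite its "running" comment.
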(event `self.ReceiveBeginPlay`
  (bind _returnvalue_x (`KismetMathLibrary.BreakVector` (`SceneComponent.K2_GetComponentLocation` (`/Game/Proteus_Multi/BP_InteractableActor.Mesh` (`self.RotationSpeedSlot`)))))
  ;[1 1 1] Save the initial position of the driller cuck and slider
  (set `self.StartLocation` (`SceneComponent.K2_GetComponentLocation` (`self.SawBladeMesh`)))
  (set `self.StartLocationSlider` _returnvalue_x)
  (set `self.NewVar_0` (`PrimitiveComponent.GetMaterial` (`self.SawBladeMesh`) 0)))

(event `self.ReceiveTick`
  (params (DeltaSeconds :type "Float (single-precision)"))
  (bind _rotationspeedslot (`self.RotationSpeedSlot`))
  (bind _returnvalue_x (`KismetMathLibrary.BreakVector` (`SceneComponent.K2_GetComponentLocation` (`/Game/Proteus_Multi/BP_InteractableActor.Mesh` (`self.RotationSpeedSlot`)))))
  (`|ExecutionSequence`
    (:`then_0`
      ;[1 1 1] Move the sawblade up and down with the lever
      (bind _asbp_interactable_actor (cast `/Game/Proteus_Multi/BP_InteractableActor` (`self.LeverSlot`)))
      (switch `/Game/Proteus_Multi/ENUM_InteractableActorType` (`/Game/Proteus_Multi/BP_InteractableActor.Type` _asbp_interactable_actor)
        (:`NewEnumerator0`
          (`SceneComponent.K2_SetWorldLocation` (`self.SawBladeMesh`) (`KismetMathLibrary.MakeVector` (.x (`self.StartLocation`)) (.y (`self.StartLocation`)) (+ (/ (`/Game/Proteus_Multi/BP_InteractableActor.CurrentAngle` _asbp_interactable_actor) 6.0) (.z (`self.StartLocation`)))) false false))))
    (:`then_1`
      ;[1 1 1] Check if Saw is ON or OFF
      (bind _asbp_interactable_actor_2 (cast `/Game/Proteus_Multi/BP_InteractableActor` (`self.ONOFFSwitchSlot`))
        (:`then`
          (switch `/Game/Proteus_Multi/ENUM_InteractableActorType` (`/Game/Proteus_Multi/BP_InteractableActor.Type` _asbp_interactable_actor_2)
            (:`NewEnumerator0`
              (set `self.ONOFF` (>= (`/Game/Proteus_Multi/BP_InteractableActor.CumulativeAngle` _asbp_interactable_actor_2) 70.0)))))
        (:`CastFailed`
          (if (`/Game/Vistom/UniversalControlls/BP_Emergency_Button.EmergencyStop` (`self.Emergency_Button`))
            (set `/Game/Vistom/UniversalControlls/BP_On_Off_Button.Run` false (`self.ONOFF_Button`))
            (set `self.ONOFF` false)
            (set `/Game/Vistom/UniversalControlls/BP_Emergency_Button.EmergencyStop` false (`self.Emergency_Button`))
            (else
              ;[1 1 1] Set on/off from Button
              (set `self.ONOFF` (`/Game/Vistom/UniversalControlls/BP_On_Off_Button.Run` (`self.ONOFF_Button`))))))))
    (:`then_2`
      ;[1 1 1] Make rotation if machine is ON
      (if (`self.ONOFF`)
        (switch `/Game/Proteus_Multi/ENUM_InteractableActorType` (`/Game/Proteus_Multi/BP_InteractableActor.Type` _rotationspeedslot)
          (:`NewEnumerator0`
            (`SceneComponent.K2_AddRelativeRotation` (`self.SawBladeMesh`) (`KismetMathLibrary.MakeRotator` 0.0 0.0 (* (+ (* (`/Game/Proteus_Multi/BP_InteractableActor.CumulativeAngle` _rotationspeedslot) 5.0) 100.0) DeltaSeconds)) false false))
          (:`NewEnumerator1`
            (`SceneComponent.K2_AddRelativeRotation` (`self.SawBladeMesh`) (`KismetMathLibrary.MakeRotator` 0.0 0.0 (* (+ (* (- _returnvalue_x (`self.StartLocationSlider`)) 20.0) 20.0) DeltaSeconds)) false false)))))
    (:`then_3`
      ;[1 1 1] Play sound when machine is running
      (if (not (`self.ONOFF`))
        (`AudioComponent.Play` (`AmbientSound.AudioComponent` (`self.Sound_Slot`)) 0.0)))))

(event `self.Box.OnComponentBeginOverlap`
  (params (OverlappedComponent :type "PrimitiveComponent Object Reference") (OtherActor :type "Actor Object Reference") (OtherComp :type "PrimitiveComponent Object Reference") (OtherBodyIndex :type Integer) (bFromSweep :type Boolean) (SweepResult :type "HitResult Structure (by ref)"))
  (cast `/Game/Proteus_Multi/MotionControllerBP` OtherActor)
  (`PrimitiveComponent.SetMaterial` (`self.SawBladeMesh`) 0 "/Game/Vistom/HandLeverCicularSaw/Materials/M_Warning.M_Warning"))

(event `self.Box.OnComponentEndOverlap`
  (params (OverlappedComponent :type "PrimitiveComponent Object Reference") (OtherActor :type "Actor Object Reference") (OtherComp :type "PrimitiveComponent Object Reference") (OtherBodyIndex :type Integer))
  (cast `/Game/Proteus_Multi/MotionControllerBP` OtherActor)
  (`PrimitiveComponent.SetMaterial` (`self.SawBladeMesh`) 0 (`self.NewVar_0`)))

(fn `UserConstructionScript`)