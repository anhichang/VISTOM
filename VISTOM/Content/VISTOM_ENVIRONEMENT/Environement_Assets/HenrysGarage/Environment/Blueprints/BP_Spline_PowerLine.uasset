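; Spline-driven power line that builds a row of BP_PowerPole child actors and their cables in the construction script.
; Poles follow spline point location, roll and yaw, and each pole's two cables snap to the next pole's connectors, with length set from distance plus random slack.
; TransfoOrNot ends the line at BP_Transfo, spawned at the last point on every loop pass; otherwise the final pole's cable lengths are zero.
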(fn `UserConstructionScript`
  (bind _numberofsplinepoints (`self.NumberOfSplinePoints`))
  (bind _spline (`self.Spline`))
  (bind _spline_2 (`self.Spline`))
  (bind _indexofloop (`self.IndexOfLoop`))
  (bind _spline_3 (`self.Spline`))
  (bind (_returnvalue_roll _returnvalue_pitch _returnvalue_yaw) (`KismetMathLibrary.BreakRotator` (`SplineComponent.GetRotationAtSplinePoint` _spline _numberofsplinepoints "Local")))
  (bind (_returnvalue_roll_2 _returnvalue_pitch_2 _returnvalue_yaw_2) (`KismetMathLibrary.BreakRotator` (`SplineComponent.GetRotationAtSplinePoint` _spline_3 _indexofloop "Local")))
  (bind _returnvalue (- (`self.IndexOfLoop`) 1))
  (bind _output (`|GetArrayItem` (`self.AllChildActorsOfPowerline`) (`self.Index Loop 2`)))
  (bind _output_2 (`|GetArrayItem` (`self.AllChildActorsOfPowerline`) (`self.NumberOfSplinePoints`)))
  (bind _output_3 (`|GetArrayItem` (`self.AllChildActorsOfPowerline`) (`self.Index Loop 2`)))
  (bind _output_4 (`|GetArrayItem` (`self.AllTransfo`) (`self.LastIndex`)))
  (bind _output_5 (`|GetArrayItem` (`self.AllChildActorsOfPowerline`) (`self.NumberOfSplinePoints`)))
  (bind (_returnvalue_roll_3 _returnvalue_pitch_3 _returnvalue_yaw_3) (`KismetMathLibrary.BreakRotator` (`SplineComponent.GetRotationAtSplinePoint` _spline_2 _returnvalue "Local")))
  (bind _output_6 (`|GetArrayItem` (`self.AllChildActorsOfPowerline`) (+ (`self.Index Loop 2`) 1)))
  (bind _output_7 (`|GetArrayItem` (`self.AllChildActorsOfPowerline`) (+ (`self.Index Loop 2`) 1)))
  (bind _cable_1 (`/Game/VISTOM_ENVIRONEMENT/Environement_Assets/HenrysGarage/Environment/Blueprints/BP_PowerPole.Cable 1` _output_5))
  (bind _cable_2 (`/Game/VISTOM_ENVIRONEMENT/Environement_Assets/HenrysGarage/Environment/Blueprints/BP_PowerPole.Cable 2` _output_5))
  (bind _cable_1_2 (`/Game/VISTOM_ENVIRONEMENT/Environement_Assets/HenrysGarage/Environment/Blueprints/BP_PowerPole.Cable 1` _output))
  (bind _cable_2_2 (`/Game/VISTOM_ENVIRONEMENT/Environement_Assets/HenrysGarage/Environment/Blueprints/BP_PowerPole.Cable 2` _output))
  (bind _cable_1_3 (`/Game/VISTOM_ENVIRONEMENT/Environement_Assets/HenrysGarage/Environment/Blueprints/BP_PowerPole.Cable 1` _output_3))
  (bind _cable_2_3 (`/Game/VISTOM_ENVIRONEMENT/Environement_Assets/HenrysGarage/Environment/Blueprints/BP_PowerPole.Cable 2` _output_3))
  (bind _con_1 (`/Game/VISTOM_ENVIRONEMENT/Environement_Assets/HenrysGarage/Environment/Blueprints/BP_Transfo.Con 1` _output_4))
  (bind _con_2 (`/Game/VISTOM_ENVIRONEMENT/Environement_Assets/HenrysGarage/Environment/Blueprints/BP_Transfo.Con 2` _output_4))
  (bind _con_1_2 (`/Game/VISTOM_ENVIRONEMENT/Environement_Assets/HenrysGarage/Environment/Blueprints/BP_PowerPole.Con 1` _output_6))
  (bind _con_2_2 (`/Game/VISTOM_ENVIRONEMENT/Environement_Assets/HenrysGarage/Environment/Blueprints/BP_PowerPole.Con 2` _output_6))
  (bind _con_1_3 (`/Game/VISTOM_ENVIRONEMENT/Environement_Assets/HenrysGarage/Environment/Blueprints/BP_PowerPole.Con 1` _output_7))
  (bind _con_2_3 (`/Game/VISTOM_ENVIRONEMENT/Environement_Assets/HenrysGarage/Environment/Blueprints/BP_PowerPole.Con 2` _output_7))
  (bind _output_get (set `self.NumberOfSplinePoints` (- (`SplineComponent.GetNumberOfSplinePoints` (`self.Spline`)) 1)))
  (if (`self.TransfoOrNot`)
    (for _index (range (+ _output_get 1))
      (set `self.IndexOfLoop` _index)
      (bind _returnvalue_2 (`AddComponent|NODE_AddChildActorComponent-3` :`RelativeTransform` (`KismetMathLibrary.Conv_VectorToTransform` (`SplineComponent.GetLocationAtSplinePoint` _spline_2 _returnvalue "Local"))))
      (`ChildActorComponent.SetChildActorClass` _returnvalue_2 "/Game/VISTOM_ENVIRONEMENT/Environement_Assets/HenrysGarage/Environment/Blueprints/BP_PowerPole.BP_PowerPole_C")
      (bind _asbp_power_pole (cast `/Game/VISTOM_ENVIRONEMENT/Environement_Assets/HenrysGarage/Environment/Blueprints/BP_PowerPole` (`ChildActorComponent.ChildActor` _returnvalue_2)))
      (`KismetArrayLibrary.Array_Add` (`self.AllChildActorsOfPowerline`) _asbp_power_pole)
      (`SceneComponent.K2_SetRelativeRotation` _returnvalue_2 (`KismetMathLibrary.MakeRotator` _returnvalue_roll_3 0.0 _returnvalue_yaw_3) false false)
      (bind _returnvalue_3 (`AddComponent|NODE_AddChildActorComponent-2` :`RelativeTransform` (`KismetMathLibrary.Conv_VectorToTransform` (`SplineComponent.GetLocationAtSplinePoint` _spline _numberofsplinepoints "Local"))))
      (`ChildActorComponent.SetChildActorClass` _returnvalue_3 "/Game/VISTOM_ENVIRONEMENT/Environement_Assets/HenrysGarage/Environment/Blueprints/BP_Transfo.BP_Transfo_C")
      (bind _asbp_transfo (cast `/Game/VISTOM_ENVIRONEMENT/Environement_Assets/HenrysGarage/Environment/Blueprints/BP_Transfo` (`ChildActorComponent.ChildActor` _returnvalue_3)))
      (`KismetArrayLibrary.Array_Add` (`self.AllTransfo`) _asbp_transfo)
      (`SceneComponent.K2_SetRelativeRotation` _returnvalue_3 (`KismetMathLibrary.MakeRotator` _returnvalue_roll 0.0 _returnvalue_yaw) false false))
    ;[1 1 1] Cable Pole to Pole
    (for _index_2 (range (+ (`self.NumberOfSplinePoints`) 1))
      (set `self.Index Loop 2` _index_2)
      (`|ExecutionSequence`
        (:`then_0`
          (`SceneComponent.K2_AttachToComponent` _cable_1_3 _con_1_3 "None" "SnapToTarget" "SnapToTarget" "KeepWorld" true)
          (set `CableComponent.CableLength` (+ (`KismetMathLibrary.VSize` (- (`SceneComponent.K2_GetComponentLocation` (`/Game/VISTOM_ENVIRONEMENT/Environement_Assets/HenrysGarage/Environment/Blueprints/BP_PowerPole.Con 1` _output_3)) (`SceneComponent.K2_GetComponentLocation` _con_1_3))) (`KismetMathLibrary.RandomFloatInRange` 0.0 80.0)) _cable_1_3)
          (`SceneComponent.K2_AttachToComponent` _cable_1 _con_1 "None" "SnapToTarget" "SnapToTarget" "KeepWorld" true)
          (set `CableComponent.CableLength` (+ (`KismetMathLibrary.VSize` (- (`SceneComponent.K2_GetComponentLocation` (`/Game/VISTOM_ENVIRONEMENT/Environement_Assets/HenrysGarage/Environment/Blueprints/BP_PowerPole.Con 1` _output_5)) (`SceneComponent.K2_GetComponentLocation` _con_1))) (`KismetMathLibrary.RandomFloatInRange` 0.0 80.0)) _cable_1))
        (:`then_1`
          (`SceneComponent.K2_AttachToComponent` _cable_2_3 _con_2_3 "None" "SnapToTarget" "SnapToTarget" "KeepWorld" true)
          (set `CableComponent.CableLength` (+ (`KismetMathLibrary.VSize` (- (`SceneComponent.K2_GetComponentLocation` (`/Game/VISTOM_ENVIRONEMENT/Environement_Assets/HenrysGarage/Environment/Blueprints/BP_PowerPole.Con 2` _output_3)) (`SceneComponent.K2_GetComponentLocation` _con_2_3))) (`KismetMathLibrary.RandomFloatInRange` 0.0 80.0)) _cable_2_3)
          (`SceneComponent.K2_AttachToComponent` _cable_2 _con_2 "None" "SnapToTarget" "SnapToTarget" "KeepWorld" true)
          (set `CableComponent.CableLength` (+ (`KismetMathLibrary.VSize` (- (`SceneComponent.K2_GetComponentLocation` (`/Game/VISTOM_ENVIRONEMENT/Environement_Assets/HenrysGarage/Environment/Blueprints/BP_PowerPole.Con 2` _output_5)) (`SceneComponent.K2_GetComponentLocation` _con_2))) (`KismetMathLibrary.RandomFloatInRange` 0.0 80.0)) _cable_2))))
    (else
      (for _index_3 (range (+ _output_get 1))
        (set `self.IndexOfLoop` _index_3)
        (bind _returnvalue_4 (`AddComponent|NODE_AddChildActorComponent-0` :`RelativeTransform` (`KismetMathLibrary.Conv_VectorToTransform` (`SplineComponent.GetLocationAtSplinePoint` _spline_3 _indexofloop "Local"))))
        (`ChildActorComponent.SetChildActorClass` _returnvalue_4 "/Game/VISTOM_ENVIRONEMENT/Environement_Assets/HenrysGarage/Environment/Blueprints/BP_PowerPole.BP_PowerPole_C")
        (bind _asbp_power_pole_2 (cast `/Game/VISTOM_ENVIRONEMENT/Environement_Assets/HenrysGarage/Environment/Blueprints/BP_PowerPole` (`ChildActorComponent.ChildActor` _returnvalue_4)))
        (`KismetArrayLibrary.Array_Add` (`self.AllChildActorsOfPowerline`) _asbp_power_pole_2)
        (`SceneComponent.K2_SetRelativeRotation` _returnvalue_4 (`KismetMathLibrary.MakeRotator` _returnvalue_roll_2 0.0 _returnvalue_yaw_2) false false))
      (for _index_4 (range (+ (`self.NumberOfSplinePoints`) 1))
        (set `self.Index Loop 2` _index_4)
        (`|ExecutionSequence`
          (:`then_0`
            (`SceneComponent.K2_AttachToComponent` _cable_1_2 _con_1_2 "None" "SnapToTarget" "SnapToTarget" "KeepWorld" true)
            (set `CableComponent.CableLength` (+ (`KismetMathLibrary.VSize` (- (`SceneComponent.K2_GetComponentLocation` (`/Game/VISTOM_ENVIRONEMENT/Environement_Assets/HenrysGarage/Environment/Blueprints/BP_PowerPole.Con 1` _output)) (`SceneComponent.K2_GetComponentLocation` _con_1_2))) (`KismetMathLibrary.RandomFloatInRange` 0.0 80.0)) _cable_1_2)
            (set `CableComponent.CableLength` 0.0 (`/Game/VISTOM_ENVIRONEMENT/Environement_Assets/HenrysGarage/Environment/Blueprints/BP_PowerPole.Cable 1` _output_2)))
          (:`then_1`
            (`SceneComponent.K2_AttachToComponent` _cable_2_2 _con_2_2 "None" "SnapToTarget" "SnapToTarget" "KeepWorld" true)
            (set `CableComponent.CableLength` (+ (`KismetMathLibrary.VSize` (- (`SceneComponent.K2_GetComponentLocation` (`/Game/VISTOM_ENVIRONEMENT/Environement_Assets/HenrysGarage/Environment/Blueprints/BP_PowerPole.Con 2` _output)) (`SceneComponent.K2_GetComponentLocation` _con_2_2))) (`KismetMathLibrary.RandomFloatInRange` 0.0 80.0)) _cable_2_2)
            (set `CableComponent.CableLength` 0.0 (`/Game/VISTOM_ENVIRONEMENT/Environement_Assets/HenrysGarage/Environment/Blueprints/BP_PowerPole.Cable 2` _output_2))))))))